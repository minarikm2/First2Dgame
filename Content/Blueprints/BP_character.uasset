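; BP_character is a playable 2D side-scrolling character with walk, sprint and jump controls.
; Enhanced Input actions add movement along world X, trigger jumps and switch max walk speed while sprint is held.
; Each tick, it picks a fall, run or idle flipbook from movement state and flips the controller yaw to face the X velocity direction.
; Movement flags are set but never cleared here.
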(event Custom|Update%20Animation
  ;[1 1 1] Is Moving or Falling
  (Sprite|SetFlipbook (Variables|Default|GetSprite) (select (AI|Components|NavMovement|IsFalling (Variables|Character|GetCharacterMovement)) "/Game/Downloads/Sunny-land-files/Sunny-land-assets-files/PNG/sprites/player/jump/FB_fall.FB_fall" (select (> (Math|Vector|VectorLength (Variables|/Script/Engine.MovementComponent|GetVelocity (Variables|Character|GetCharacterMovement))) 0.0) "/Game/Downloads/Sunny-land-files/Sunny-land-assets-files/PNG/sprites/player/run/FB_run.FB_run" "/Game/Downloads/Sunny-land-files/Sunny-land-assets-files/PNG/sprites/player/idle/FB_chill.FB_chill")))
  (Variables|Default|SetIsMoving true))

(event Custom|Update%20Control%20Rotation
  ;[1 1 1] Side Moving
  (Utilities|IsValid (Pawn|GetController)
    (:Is%20Valid
      (Math|Float|CompareFloat (.X (Math|Vector|BreakVector (Variables|/Script/Engine.MovementComponent|GetVelocity (Variables|Character|GetCharacterMovement)))) 0.0
        (:>
          (Pawn|SetControlRotation (Pawn|GetController) (Math|Rotator|MakeRotator 0.0 0.0 0.0))
          (Variables|Default|SetIsMovingRight true))
        (:<
          (Pawn|SetControlRotation (Pawn|GetController) (Math|Rotator|MakeRotator 0.0 0.0 1.8e+02))
          (Variables|Default|SetIsMovingLeft true))))))

(event Input|EnhancedActionEvents|EnhancedInputActionIA_MoveForward
  (params (ActionValue :type Boolean) (ElapsedSeconds :type Float%20%28double-precision%29) (TriggeredSeconds :type Float%20%28double-precision%29) (InputAction :type Input%20Action%20Object%20Reference :default "/Game/Input/Actions/IA_MoveForward.IA_MoveForward"))
  ;[1 1 1] LOCOmotion
  (:Triggered
    (Pawn|Input|AddMovementInput "1.000000,0.000000,0.000000" 1.0 false :!label _label))
  (:Started
    (goto _label))
  (:Ongoing
    (goto _label)))

(event Input|EnhancedActionEvents|EnhancedInputActionIA_MoveBack
  (params (ActionValue :type Boolean) (ElapsedSeconds :type Float%20%28double-precision%29) (TriggeredSeconds :type Float%20%28double-precision%29) (InputAction :type Input%20Action%20Object%20Reference :default "/Game/Input/Actions/IA_MoveBack.IA_MoveBack"))
  ;[1 1 1] LOCOmotion
  (:Triggered
    (Pawn|Input|AddMovementInput "-1.000000,0.000000,0.000000" 1.0 false :!label _label))
  (:Started
    (goto _label))
  (:Ongoing
    (goto _label)))

(event Input|EnhancedActionEvents|EnhancedInputActionIA_Jump
  (params (ActionValue :type Boolean) (ElapsedSeconds :type Float%20%28double-precision%29) (TriggeredSeconds :type Float%20%28double-precision%29) (InputAction :type Input%20Action%20Object%20Reference :default "/Game/Input/Actions/IA_Jump.IA_Jump"))
  ;[1 1 1] LOCOmotion
  (:Triggered
    (Character|Jump :!label _label))
  (:Started
    (goto _label))
  (:Ongoing
    (goto _label))
  (:Completed
    (Character|StopJumping)))

(event Input|EnhancedActionEvents|EnhancedInputActionIA_SpeedRun
  (params (ActionValue :type Boolean) (ElapsedSeconds :type Float%20%28double-precision%29) (TriggeredSeconds :type Float%20%28double-precision%29) (InputAction :type Input%20Action%20Object%20Reference :default "/Game/Input/Actions/IA_SpeedRun.IA_SpeedRun"))
  ;[1 1 1] LOCOmotion
  (:Triggered
    (Variables|/Script/Engine.CharacterMovementComponent|SetMaxWalkSpeed (Variables|Character|GetCharacterMovement) 3.5e+02 :!label _label))
  (:Started
    (goto _label))
  (:Ongoing
    (goto _label))
  (:Canceled
    (Variables|/Script/Engine.CharacterMovementComponent|SetMaxWalkSpeed (Variables|Character|GetCharacterMovement) 1.5e+02 :!label _label_2))
  (:Completed
    (goto _label_2)))

(event EventTick
  (params (DeltaSeconds :type Float%20%28single-precision%29))
  ;[1 1 1] Default - thicking
  (CallFunction|UpdateAnimation)
  (CallFunction|UpdateControlRotation))

(fn ConstructionScript)